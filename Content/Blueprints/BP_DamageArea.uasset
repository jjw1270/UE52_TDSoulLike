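; BP_DamageArea is a placeable area actor that periodically damages pawns standing inside its box.
; On BeginPlay it starts a looping timer that runs a box overlap query for pawns at the Box component's location and extent.
; Each pawn with an Ability System Component applies a GE_Damage spec to itself, with the Damage variable passed as a SetByCaller magnitude.
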(event Custom|DamageTimer
  (bind _box (Variables|Default|GetBox))
  (bind _outactors (Collision|BoxOverlapActors (Transformation|GetWorldLocation _box) (Variables|/Script/Engine.BoxComponent|GetBoxExtent _box) (Utilities|Array|MakeArray "ObjectTypeQuery3") 0 :!class /Script/Engine.KismetSystemLibrary))
  (for _array_element _outactors
    (Utilities|IsValid (Ability|GetAbilitySystemComponent _array_element)
      (:Is%20Valid
        (bind _returnvalue (Ability|GameplayEffect|AssignTagSetbyCallerMagnitude (GameplayEffects|MakeOutgoingSpec (Ability|GetAbilitySystemComponent _array_element) "/Game/GAS/Effects/GE_Damage.GE_Damage_C" 0.0 (GameplayEffects|MakeEffectContext (Ability|GetAbilitySystemComponent _array_element))) "(TagName=\"Damage.SetByCaller\")" (Variables|Default|GetDamage)))
        (GameplayEffects|ApplyGameplayEffectSpecToSelf (Ability|GetAbilitySystemComponent _array_element) _returnvalue)))))

(event EventBeginPlay
  (Utilities|Time|SetTimerbyEvent (delegate Custom|DamageTimer) 0.5 true))

(event Collision|EventActorBeginOverlap
  (params (OtherActor :type Actor%20Object%20Reference)))

(event EventTick
  (params (DeltaSeconds :type Float%20%28single-precision%29)))

(fn ConstructionScript)