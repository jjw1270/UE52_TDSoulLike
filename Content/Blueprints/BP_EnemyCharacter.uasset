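; Enemy character Blueprint that reacts to Gameplay Ability System attribute changes, with debug behavior built in.
; Health and armor changes print the new value and delta.
; Rising chill slows the enemy through CustomTimeDilation, and at the threshold stops its time entirely and applies the freeze debuff effect to itself.
; Every Tick it calls Jump and prints an attribute value read from its AbilitySystemComponent.
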(event EventBeginPlay)

(event Collision|EventActorBeginOverlap
  (params (OtherActor :type Actor%20Object%20Reference)))

(event EventTick
  (params (DeltaSeconds :type Float%20%28single-precision%29))
  (Character|Jump)
  (Development|PrintString (Utilities|String|ToString(Float) (.ReturnValue (Ability|Attribute|GetFloatAttributefromAbilitySystemComponent (Variables|Default|GetAbilitySystemComponent) "(AttributeName=\"Chilled\",Attribute=/Script/TDSoulLike.TDSAttributeSet:Chilled,AttributeOwner=/Script/CoreUObject.Class'\"/Script/TDSoulLike.TDSAttributeSet\"')"))) true false "(R=0.000000,G=0.660000,B=1.000000,A=1.000000)" 0.0))

(event EventOnHealthChanged
  (params (OldValue :type Float%20%28single-precision%29) (NewValue :type Float%20%28single-precision%29))
  (Development|PrintString (Utilities|String|Append "Health - " (Utilities|String|ToString(Float) NewValue) ", " (Utilities|String|ToString(Float) (- NewValue OldValue)))))

(event EventOnArmorChanged
  (params (OldValue :type Float%20%28single-precision%29) (NewValue :type Float%20%28single-precision%29))
  (Development|PrintString (Utilities|String|Append "Armor - " (Utilities|String|ToString(Float) NewValue) ", " (Utilities|String|ToString(Float) (- NewValue OldValue)))))

(event EventOnChilledChanged
  (params (OldValue :type Float%20%28single-precision%29) (NewValue :type Float%20%28single-precision%29))
  (Variables|Default|SetCustomTimeDilation (Math|Float|MapRangeClamped NewValue 0.0 1e+02 1.0 0.5))
  (if (>= NewValue 1e+02)
    (Variables|Default|SetCustomTimeDilation 0.0)
    (GameplayEffects|ApplyGameplayEffectToSelf :self (Variables|Default|GetAbilitySystemComponent) :GameplayEffectClass "/Game/GAS/Effects/GE_Debuff_Freeze.GE_Debuff_Freeze_C")))

(fn ConstructionScript)