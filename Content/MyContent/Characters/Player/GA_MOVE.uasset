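; Gameplay Ability for cursor-driven movement of the player character.
; While the input is held, a looping WaitDelay task repeatedly traces under the cursor, caches the hit location and adds movement input toward it, printing a debug string each pass.
; Input release ends the ability, and OnEndAbility calls SimpleMoveToLocation to the cached destination and spawns a cursor effect there.
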(event Ability|EventActivateAbility
  (bind _astdslplayer_character (Utilities|Casting|CastToTDSLPlayerCharacter (Ability|GetAvatarActorfromActorInfo)))
  (bind _output_get (Variables|Default|SetPlayerCharacter _astdslplayer_character))
  (bind _asbp_tdslplayer_controller (Utilities|Casting|CastToBP_TDSLPlayerController (Pawn|GetController _output_get)))
  (Variables|Default|SetPlayerController _asbp_tdslplayer_controller)
  (Ability|Tasks|WaitInputRelease true
    (:then
      (Ability|Tasks|WaitDelay 0.001 :!label _label
        (:OnFinish
          (Development|PrintString "Hello")
          (CallFunction|Moveto (Variables|Default|GetPlayerController))
          (goto _label))))
    (:OnRelease
      (Ability|EndAbility))))

(event Ability|EventOnEndAbility
  (params (bWasCancelled :type Boolean))
  (bind _cacheddestination (Variables|Default|GetCachedDestination))
  (bind _astdslplayer_character (Utilities|Casting|CastToTDSLPlayerCharacter (Ability|GetAvatarActorfromActorInfo)))
  (bind _output_get (Variables|Default|SetPlayerCharacter _astdslplayer_character))
  (bind _asbp_tdslplayer_controller (Utilities|Casting|CastToBP_TDSLPlayerController (Pawn|GetController _output_get)))
  (AI|Navigation|SimpleMovetoLocation _asbp_tdslplayer_controller _cacheddestination)
  (Niagara|SpawnSystematLocation "/Game/Cursor/FX_Cursor.FX_Cursor" _cacheddestination))

(fn Moveto
  (params (PC :type BP%20TDSL%20Player%20Controller%20Object%20Reference))
  (bind (_hitresult _returnvalue) (Game|Player|GetHitResultUnderCursorbyChannel PC "TraceTypeQuery1" true))
  (bind _playercharacter (Variables|Default|GetPlayerCharacter))
  (if _returnvalue
    (bind _output_get (Variables|Default|SetCachedDestination (.Location (Collision|BreakHitResult _hitresult))))
    (Pawn|Input|AddMovementInput _playercharacter (Math|Vector|Normalize (- _output_get (Transformation|GetActorLocation _playercharacter))) 1.0 false)))