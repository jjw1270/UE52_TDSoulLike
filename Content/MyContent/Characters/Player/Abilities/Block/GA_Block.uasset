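; Player block ability that opens with a short parry window, then swaps the parrying effect for a blocking effect until input release.
; Activation requires sufficient stamina, stops movement and turns the player toward the cursor.
; Received hits turn the player toward the attacker and play an impact montage with root-motion knockback, adding a parry cue while the delay task is valid.
; A hit with no stamina plays a guard-break montage and ends the ability.
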(event Ability|EventActivateAbility
  (bind _returnvalue (Ability|GetAbilityLevel))
  (bind _returnvalue_2 (Ability|CommitAbility))
  (if _returnvalue_2
    (bind _returnvalue_3 (CallFunction|CheckStaminaRemain 0.2))
    (if _returnvalue_3
      ;[1 1 1] Parrying in few sec
      (bind _returnvalue_4 (Ability|ApplyGameplayEffectToOwner "/Game/MyContent/Characters/Player/Abilities/Block/GE_Parrying.GE_Parrying_C" _returnvalue))
      (bind _output_get (Variables|Default|SetGEParrying _returnvalue_4))
      (bind _asynctaskproxy (Ability|Tasks|WaitDelay 0.5)
        (:then
          (Variables|Default|SetParryingTask _asynctaskproxy)
          (Class|TDSLGameplayAbility|StopActorMovement)
          (Class|TDSLGameplayAbility|SetPlayerRotationtoUnderCursor true 15.0)
          (Ability|Tasks|WaitInputRelease false
            (:then
              (bind (_asynctaskproxy_2 _sourceasc) (|WaitReceiveDamage false)
                (:then
                  (Variables|Default|SetWaitReceiveDamage _asynctaskproxy_2))
                (:OnDamage
                  (Utilities|SetRottoDamagingSource _sourceasc)
                  (bind _returnvalue_5 (CallFunction|CheckStaminaRemain 0.0))
                  (if _returnvalue_5
                    (Variables|Default|GetParryingTask
                      (:then
                        (Utilities|FlowControl|Sequence
                          (:then_0
                            (GameplayCue|AddGameplayCue :GameplayCueTag "(TagName=\"GameplayCue.Player.Parrying\")")
                            (Utilities|FlowControl|Delay 0.2)
                            (GameplayCue|RemoveGameplayCue "(TagName=\"GameplayCue.Player.Parrying\")"))
                          (:then_1
                            (bind _blockingmontagetask (Variables|Default|GetBlockingMontageTask :!label _label)
                              (:then
                                (GameplayTasks|EndTask _blockingmontagetask))
                              (:else
                                _))
                            (bind _asynctaskproxy_3 (|PlayMontageandWaitProxy "None" "/Game/Characters/Paladin/Amimation/Blocking/AM_BlockingImpact.AM_BlockingImpact" 1.0 "None" false 1.0 0.1)
                              (:then
                                (Variables|Default|SetBlockingMontageTask _asynctaskproxy_3)
                                (Utilities|ApplyRootMotionConstForce 7e+02 0.1))))))
                      (:else
                        (goto _label)))
                    (else
                      (|PlayMontageandWaitProxy "None" "/Game/Characters/Paladin/Amimation/AM_OnOutOfBlock.AM_OnOutOfBlock" 1.0 "None" false 1.0 0.1
                        (:then
                          (Utilities|ApplyRootMotionConstForce 7e+02 0.3)
                          (Ability|EndAbility))))))))
            (:OnRelease
              (Ability|EndAbility))))
        (:OnFinish
          (Ability|RemoveGameplayEffectFromOwnerWithHandle _output_get)
          (bind _returnvalue_6 (Ability|ApplyGameplayEffectToOwner "/Game/MyContent/Characters/Player/Abilities/Block/GE_Block.GE_Block_C" _returnvalue))
          (Variables|Default|SetGEBlock _returnvalue_6)))
      (else
        (Ability|CancelAbility :!label _label_2)))
    (else
      (goto _label_2))))

(event Ability|EventOnEndAbility
  (params (bWasCancelled :type Boolean))
  (Ability|RemoveGameplayEffectFromOwnerWithHandle (Variables|Default|GetGEBlock))
  (bind _parryingtask (Variables|Default|GetParryingTask)
    (:then
      (GameplayTasks|EndTask _parryingtask)
      (Ability|RemoveGameplayEffectFromOwnerWithHandle (Variables|Default|GetGEParrying)))
    (:else
      _))
  (bind _waitreceivedamage (Variables|Default|GetWaitReceiveDamage)
    (:then
      (GameplayTasks|EndTask _waitreceivedamage))
    (:else)))

(fn CheckStaminaRemain
  (params (RemainPercent :type Float%20%28double-precision%29))
  (bind _returnvalue (Ability|GetOwningActorfromActorInfo))
  (return (> (/ (.ReturnValue (Ability|Attribute|GetFloatAttribute _returnvalue "(AttributeName=\"BlockGage\",Attribute=/Script/TDSoulLike.TDSLAttributeSetBase:BlockGage,AttributeOwner=/Script/CoreUObject.Class'\"/Script/TDSoulLike.TDSLAttributeSetBase\"')")) (.ReturnValue (Ability|Attribute|GetFloatAttribute _returnvalue "(AttributeName=\"MaxBlockGage\",Attribute=/Script/TDSoulLike.TDSLAttributeSetBase:MaxBlockGage,AttributeOwner=/Script/CoreUObject.Class'\"/Script/TDSoulLike.TDSLAttributeSetBase\"')"))) RemainPercent)))