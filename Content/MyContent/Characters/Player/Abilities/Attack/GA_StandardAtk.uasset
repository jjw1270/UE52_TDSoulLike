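; Player standard attack Gameplay Ability that plays a four-step melee combo.
; The GE_StackAtk count selects the montage and lunge; stacks clear when GE_WaitAtk is absent or the count falls outside the combo.
; Each attack adds a stack, turns the player toward the cursor and applies a pulse-out root motion force.
; GE_WaitAtk marks the combo window, and the ability ends when the montage completes.
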(event Ability|EventActivateAbility
  (bind _returnvalue (Ability|GetAbilitySystemComponentfromActorInfo))
  (bind _returnvalue_2 (GameplayEffects|GetGameplayEffectCount _returnvalue "/Game/MyContent/Characters/Player/Abilities/Attack/GE_StackAtk.GE_StackAtk_C" 0 true))
  (bind _returnvalue_3 (Ability|CommitAbility))
  (if _returnvalue_3
    (Class|TDSLGameplayAbility|StopActorMovement)
    (Utilities|IsComboRemain
      (:True
        (switch int _returnvalue_2 :!label _label
          (:Default
            (Ability|RemoveGameplayEffectFromOwnerWithGrantedTags "(GameplayTags=((TagName=\"State.AtkStack\")))" _returnvalue_2 :!label _label_2)
            (goto _label))
          (:0
            (Utilities|Attack (Variables|Default|GetAtk1) 0.0 0.0))
          (:1
            (Utilities|Attack (Variables|Default|GetAtk2) 1.5e+02 0.4))
          (:2
            (Utilities|Attack (Variables|Default|GetAtk3) 1e+02 1.0))
          (:3
            (Utilities|Attack (Variables|Default|GetAtk4) 1e+02 1.0))))
      (:False
        (goto _label_2)))
    (Ability|EndAbility)
    (else
      (Ability|CancelAbility))))

(event Ability|EventOnEndAbility
  (params (bWasCancelled :type Boolean))
  (bind _montagetask (Variables|Default|GetMontageTask)
    (:then
      (GameplayTasks|EndTask _montagetask))
    (:else)))