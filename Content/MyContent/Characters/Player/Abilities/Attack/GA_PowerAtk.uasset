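; Player power attack ability that picks its montage from the current GE_StackAtk combo count.
; On activation it stops movement and clears the stacks if no GE_WaitAtk combo window is active.
; Stacks 3 and 4 add two stacks to chain into follow-up montages, while other cases consume the stacks.
; The Attack graph turns toward the cursor, plays the montage, applies forward root-motion force and grants GE_WaitAtk.
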(event Ability|EventActivateAbility
  (bind _returnvalue (Ability|GetAbilitySystemComponentfromActorInfo))
  (bind _returnvalue_2 (GameplayEffects|GetGameplayEffectCount _returnvalue "/Game/MyContent/Characters/Player/Abilities/Attack/GE_StackAtk.GE_StackAtk_C" 0 true))
  (bind _returnvalue_3 (Ability|CommitAbility))
  (if _returnvalue_3
    (Class|TDSLGameplayAbility|StopActorMovement)
    (Utilities|IsComboRemain
      (:True
        _)
      (:False
        (Ability|RemoveGameplayEffectFromOwnerWithGrantedTags "(GameplayTags=((TagName=\"State.AtkStack\")))" _returnvalue_2)))
    (switch int _returnvalue_2
      (:0
        (Utilities|Attack (Variables|Default|GetAtk0) _returnvalue_2 0.0 0.0 false))
      (:1
        (Utilities|Attack (Variables|Default|GetAtk1) _returnvalue_2 0.0 0.0 false))
      (:2
        (Utilities|Attack (Variables|Default|GetAtk2) _returnvalue_2 6e+02 2.0 false))
      (:3
        (Utilities|Attack (Variables|Default|GetAtk3) 0 2e+02 0.3 true))
      (:4
        (Utilities|Attack (Variables|Default|GetAtk4) 0 4e+02 0.6 true))
      (:5
        (Utilities|Attack (Variables|Default|GetAtk3_2) _returnvalue_2 3e+02 2.0 false))
      (:6
        (Utilities|Attack (Variables|Default|GetAtk4_2) _returnvalue_2 2e+02 3.2 false)))
    (Ability|EndAbility)
    (else
      (Ability|CancelAbility))))

(event Ability|EventOnEndAbility
  (params (bWasCancelled :type Boolean))
  (bind _montagetask (Variables|Default|GetMontageTask)
    (:then
      (GameplayTasks|EndTask _montagetask))
    (:else)))