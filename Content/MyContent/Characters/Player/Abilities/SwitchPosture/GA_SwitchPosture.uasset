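; Gameplay Ability that toggles the player character between Normal and Battle postures.
; After committing, it checks the ability system for an active GE_NormalPose effect to pick the target posture.
; It removes the opposite posture's effect by granted tag, applies the new posture effect and plays its montage.
; The ability ends immediately without waiting for the montage, or cancels if the commit fails.
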(event Ability|EventActivateAbility
  (bind _asbp_tdslplayer_character (Utilities|Casting|CastToBP_TDSLPlayerCharacter (Ability|GetAvatarActorfromActorInfo)))
  (Variables|Default|SetPlaye%20Character _asbp_tdslplayer_character)
  (bind _returnvalue (Ability|CommitAbility))
  (if _returnvalue
    (if (== (GameplayEffects|GetGameplayEffectCount (Ability|GetAbilitySystemComponentfromActorInfo) "/Game/MyContent/Characters/Player/Effects/SwitchPosture/GE_NormalPose.GE_NormalPose_C" 0 true) 0)
      (Ability|RemoveGameplayEffectFromOwnerWithGrantedTags "(GameplayTags=((TagName=\"State.Posture.Battle\")))")
      (Ability|ApplyGameplayEffectToOwner "/Game/MyContent/Characters/Player/Effects/SwitchPosture/GE_NormalPose.GE_NormalPose_C")
      (Animation|PlayAnimMontage (Variables|Default|GetPlaye%20Character) "/Game/Characters/Paladin/Amimation/AM_OnNormal.AM_OnNormal" 1.0 "None")
      (else
        (Ability|RemoveGameplayEffectFromOwnerWithGrantedTags "(GameplayTags=((TagName=\"State.Posture.Normal\")))")
        (Ability|ApplyGameplayEffectToOwner "/Game/MyContent/Characters/Player/Effects/SwitchPosture/GE_BattlePose.GE_BattlePose_C")
        (Animation|PlayAnimMontage (Variables|Default|GetPlaye%20Character) "/Game/Characters/Paladin/Amimation/AM_OnBattle.AM_OnBattle" 1.0 "None")))
    (Ability|EndAbility)
    (else
      (Ability|CancelAbility))))

(event Ability|EventOnEndAbility
  (params (bWasCancelled :type Boolean)))