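; Gameplay ability that handles cursor-driven, click-to-move control of the player.
; While input is held, a short WaitDelay loop prints a debug string and calls MoveTo, which traces under the cursor, caches the hit and adds movement input toward it.
; Releasing input ends the ability.
; On end, SimpleMoveToLocation sends the controller to the cached destination and a cursor effect spawns there.
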(event Ability|EventActivateAbility
  (Ability|Tasks|WaitInputRelease true
    (:then
      (Ability|Tasks|WaitDelay 0.005 :!label _label
        (:OnFinish
          (Development|PrintString "Moving" true false "(R=1.000000,G=0.475625,B=0.290296,A=1.000000)" 0.005)
          (CallFunction|Moveto)
          (goto _label))))
    (:OnRelease
      (Ability|EndAbility))))

(event Ability|EventOnEndAbility
  (params (bWasCancelled :type Boolean))
  (bind _cacheddestination (Variables|Default|GetCachedDestination))
  (AI|Navigation|SimpleMovetoLocation (.PlayerController (Utilities|Struct|BreakGameplayAbilityActorInfo (Ability|GetActorInfo))) _cacheddestination)
  (Niagara|SpawnSystematLocation (Variables|Default|GetFXCursor) _cacheddestination))

(fn Moveto
  (bind _returnvalue (Ability|GetActorInfo))
  (bind _returnvalue_2 (Ability|GetAvatarActorfromActorInfo))
  (bind _playercontroller (Utilities|Struct|BreakGameplayAbilityActorInfo _returnvalue))
  (bind _hitresult (Game|Player|GetHitResultUnderCursorbyChannel _playercontroller "TraceTypeQuery1" true))
  (bind (_bblockinghit _binitialoverlap _time _distance _location) (Collision|BreakHitResult _hitresult))
  (if _bblockinghit
    (bind _output_get (Variables|Default|SetCachedDestination _location))
    (Pawn|Input|AddMovementInput (Variables|/Script/Engine.Actor|GetInstigator _returnvalue_2) (Math|Vector|GetUnitDirection(Vector) (Transformation|GetActorLocation _returnvalue_2) _output_get) 1.0 false)))