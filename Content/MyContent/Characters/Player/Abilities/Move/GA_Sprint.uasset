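; Gameplay ability that makes the player sprint while input is held, starting only when a ratio of two owner attributes exceeds 0.2.
; It applies GE_Sprint and starts sprinting on the custom TDSL movement component.
; A short, net-synced delay loop recommits the ability while the character accelerates on the ground, ending it otherwise or on input release.
; Ending removes the effect and stops sprinting.
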(event Ability|EventActivateAbility
  (bind _returnvalue (Ability|GetOwningActorfromActorInfo))
  (if (> (/ (.ReturnValue (Ability|Attribute|GetFloatAttribute _returnvalue "(AttributeName=\"Stamina\",Attribute=/Script/TDSoulLike.TDSLAttributeSetBase:Stamina,AttributeOwner=/Script/CoreUObject.Class'\"/Script/TDSoulLike.TDSLAttributeSetBase\"')")) (.ReturnValue (Ability|Attribute|GetFloatAttribute _returnvalue "(AttributeName=\"MaxStamina\",Attribute=/Script/TDSoulLike.TDSLAttributeSetBase:MaxStamina,AttributeOwner=/Script/CoreUObject.Class'\"/Script/TDSoulLike.TDSLAttributeSetBase\"')"))) 0.2)
    (bind _returnvalue_2 (Ability|ApplyGameplayEffectToOwner "/Game/MyContent/Characters/Player/Abilities/Move/GE_Sprint.GE_Sprint_C" (Ability|GetAbilityLevel)))
    (Variables|Default|SetGESprint _returnvalue_2)
    (bind _astdslcharacter_movement_component (Utilities|Casting|CastToTDSLCharacterMovementComponent (.MovementComponent (Utilities|Struct|BreakGameplayAbilityActorInfo (Ability|GetActorInfo)))))
    (bind _output_get (Variables|Default|SetCharacterMovementComp _astdslcharacter_movement_component))
    (Class|TDSLCharacterMovementComponent|StartSprinting _output_get)
    (Ability|Tasks|WaitInputRelease false
      (:then
        (Ability|Tasks|WaitDelay 0.05 :!label _label
          (:OnFinish
            (Ability|Tasks|WaitNetSync "OnlyServerWait"
              (:OnSync
                (if (and (> (Math|Vector|VectorLength (Pawn|Components|CharacterMovement|GetCurrentAcceleration (Variables|Default|GetCharacterMovementComp))) 0.0) (not (AI|Components|NavMovement|IsFalling (Variables|Default|GetCharacterMovementComp))))
                  (bind _returnvalue_3 (Ability|CommitAbility))
                  (if _returnvalue_3
                    (goto _label)
                    (else
                      _)))
                (Ability|EndAbility))))))
      (:OnRelease
        (Ability|EndAbility)))
    (else
      (Ability|EndAbility))))

(event Ability|EventOnEndAbility
  (params (bWasCancelled :type Boolean))
  (bind _charactermovementcomp (Variables|Default|GetCharacterMovementComp))
  (Ability|RemoveGameplayEffectFromOwnerWithHandle (Variables|Default|GetGESprint))
  (Utilities|IsValid _charactermovementcomp
    (:Is%20Valid
      (Class|TDSLCharacterMovementComponent|StopSprinting _charactermovementcomp))))