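; AI controller for the boss enemy that runs the BT_BossAI behavior tree on BeginPlay.
; When AI perception successfully senses an actor, it stores that actor as TargetActor in the blackboard and sets AIState to Chase.
; Losing perception changes nothing, as the nodes that would reset the target and state are disconnected, and a debug "Hello" print remains on detection.
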(event OnTargetPerceptionUpdated(AIPerception)
  (params (Actor :type Actor%20Object%20Reference) (Stimulus :type AI%20Stimulus%20Structure))
  (if (.bSuccessfullySensed (Utilities|Struct|BreakAIStimulus Stimulus))
    (Development|PrintString "Hello")
    (AI|Components|Blackboard|SetValueasObject (Variables|Default|GetBlackboard) (Utilities|Name|MakeLiteralName "TargetActor") Actor)
    (AI|Components|Blackboard|SetValueasEnum (Variables|Default|GetBlackboard) (Utilities|Name|MakeLiteralName "AIState") (Utilities|Enum|LiteralenumEEnemyAIState "Chase"))))

(event EventBeginPlay
  (AI|RunBehaviorTree "/Game/MyContent/AI/Boss/BT_BossAI.BT_BossAI"))

(fn ConstructionScript)