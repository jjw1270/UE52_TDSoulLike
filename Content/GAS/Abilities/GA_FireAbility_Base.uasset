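; Base gameplay ability that fires a projectile from the top-down character, either once or repeatedly in full-auto.
; Activation commits the ability and fires; full-auto then loops on a rate-of-fire delay, re-committing before each shot until input release or a failed commit ends it.
; Each shot spawns the projectile ahead of the character, passing it a gameplay effect spec with set-by-caller damage and a damage tag.
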(event Ability|EventActivateAbility
  (bind _asbp_top_down_character (Utilities|Casting|CastToBP_TopDownCharacter (Ability|GetAvatarActorfromActorInfo)))
  (Variables|Default|SetCharacter _asbp_top_down_character)
  (Ability|CommitAbility)
  (CallFunction|Fire)
  (if (Variables|Default|GetIsFullAuto)
    (Ability|Tasks|WaitInputRelease false
      (:then
        (GameplayTasks|TaskWaitDelay 0 (/ 1.0 (Variables|Default|GetRateOfFire)) :!label _label
          (:OnFinish
            (bind _returnvalue (Ability|CommitAbility))
            (if _returnvalue
              (CallFunction|Fire)
              (goto _label)
              (else
                (Ability|EndAbility))))))
      (:OnRelease
        (Ability|EndAbility)))
    (else
      (Ability|EndAbility))))

(event Ability|EventOnEndAbility
  (params (bWasCancelled :type Boolean)))

(fn MakeSpec
  (bind _character (Variables|Default|GetCharacter)
    (:then
      (bind _returnvalue (Ability|GameplayEffect|AssignTagSetbyCallerMagnitude (GameplayEffects|MakeOutgoingSpec (Ability|GetAbilitySystemComponent _character) (Variables|Default|GetGameplayEffectClass) 0.0 (GameplayEffects|MakeEffectContext (Ability|GetAbilitySystemComponent _character))) "(TagName=\"Damage.SetByCaller\")" (Variables|Default|GetDamage)))
      (bind _returnvalue_2 (Ability|GameplayEffect|AddAssetTag _returnvalue (Variables|Default|GetDamageTag)))
      (return _returnvalue_2))
    (:else)))

(fn Fire
  (bind _character (Variables|Default|GetCharacter))
  (bind _spechandle (CallFunction|MakeSpec))
  (Game|SpawnActorfromClass (Variables|Default|GetProjectileClass) (Math|Transform|MakeTransform (+ (Transformation|GetActorLocation _character) (* (Transformation|GetActorForwardVector _character) 1e+02)) (Transformation|GetActorRotation _character) "0.400000,0.400000,0.400000") "Undefined" "MultiplyWithRoot" (Variables|Default|GetCharacter) _spechandle 0))