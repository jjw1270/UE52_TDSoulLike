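; GA_DashAbility is a gameplay ability that, despite its name, fires a projectile from the BP_TopDownCharacter avatar and contains no dash movement.
; On activation it commits, builds a GE_Damage spec with the Damage value set through a SetByCaller tag, and passes it to a scaled-down BP_Projectile spawned ahead of the character.
; The ability ends immediately after spawning, and an input-release wait with a debug print is left unconnected.
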(event Ability|EventActivateAbility
  (bind _returnvalue (Ability|GetAvatarActorfromActorInfo))
  (Development|PrintString "Dash Ability")
  (Ability|CommitAbility)
  (bind _asbp_top_down_character (Utilities|Casting|CastToBP_TopDownCharacter _returnvalue))
  (bind _returnvalue_2 (Ability|GameplayEffect|AssignTagSetbyCallerMagnitude (GameplayEffects|MakeOutgoingSpec (Ability|GetAbilitySystemComponent _asbp_top_down_character) "/Game/GAS/Effects/GE_Damage.GE_Damage_C" 0.0 (GameplayEffects|MakeEffectContext (Ability|GetAbilitySystemComponent _asbp_top_down_character))) "(TagName=\"Damage.SetByCaller\")" (Variables|Default|GetDamage)))
  (Game|SpawnActorfromClass "/Game/Blueprints/BP_Projectile.BP_Projectile_C" (Math|Transform|MakeTransform (+ (Transformation|GetActorLocation _asbp_top_down_character) (* (Transformation|GetActorForwardVector _asbp_top_down_character) 1e+02)) (Transformation|GetActorRotation _asbp_top_down_character) "0.400000,0.400000,0.400000") "Undefined" "MultiplyWithRoot" _returnvalue _returnvalue_2 0)
  (Ability|EndAbility))

(event Ability|EventOnEndAbility
  (params (bWasCancelled :type Boolean)))